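; AC_ZMovable is an actor component that gives its owner stepped vertical positions along Z.
; On BeginPlay it stores the owner's starting Z as a base and snaps the owner to the height of the current step.
; Up and Down change the step within a clamped range and recompute the target height from the step size, without moving the actor themselves.
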(event `self.ReceiveBeginPlay`
  (bind _returnvalue (`self.GetOwner`))
  (bind (_returnvalue_x _returnvalue_y _returnvalue_z) (`KismetMathLibrary.BreakVector` (`Actor.K2_GetActorLocation` _returnvalue)))
  ;[1 0.5052 0.5052] Inicialización
  (bind _output_get (set `self.Initial` _returnvalue_z))
  (bind _output_get_2 (set `self.Target` (+ _output_get (* (`self.ActualStep`) (`self.StepSize`)))))
  (`Actor.K2_SetActorLocation` _returnvalue (`KismetMathLibrary.MakeVector` _returnvalue_x _returnvalue_y _output_get_2) false false))

(fn `Down`
  (params (Steps :type Integer))
  (bind _output_get (set `self.ActualStep` (`KismetMathLibrary.Max` (+ (* -1 Steps) (`self.ActualStep`)))))
  (set `self.Target` (+ (* _output_get (`self.StepSize`)) (`self.Initial`)))
  (return))

(fn `Up`
  (params (Steps :type Integer))
  (bind _output_get (set `self.ActualStep` (`KismetMathLibrary.Min` (+ Steps (`self.ActualStep`)) 15)))
  (set `self.Target` (+ (* _output_get (`self.StepSize`)) (`self.Initial`)))
  (return))