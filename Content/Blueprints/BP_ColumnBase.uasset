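; BP_ColumnBase is a base Blueprint for a column with an attached stair that can move vertically.
; MoveStairAndColumn takes a height and a direction flag and calls Up or Down on the ACZMovable component of both the Stair and the Column, so the two shift together by the same amount.
; The construction script is empty.
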(fn `MoveStairAndColumn`
  (params (Height :type Integer) (IsUp :type Boolean))
  (bind _ac_zmovable (`/Game/Blueprints/BP_Stair.AC_ZMovable` (`self.Stair`)))
  (bind _ac_zmovable_2 (`/Game/Blueprints/BP_Column.AC_ZMovable` (`self.Column`)))
  (if IsUp
    (`|ExecutionSequence`
      (:`then_0`
        (`/Game/Blueprints/AC_ZMovable.Up` _ac_zmovable Height))
      (:`then_1`
        (`/Game/Blueprints/AC_ZMovable.Up` _ac_zmovable_2 Height)))
    (else
      (`|ExecutionSequence`
        (:`then_0`
          (`/Game/Blueprints/AC_ZMovable.Down` _ac_zmovable Height))
        (:`then_1`
          (`/Game/Blueprints/AC_ZMovable.Down` _ac_zmovable_2 Height))))))

(fn `UserConstructionScript`)