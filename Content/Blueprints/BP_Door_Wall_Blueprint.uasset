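; BP_Door_Wall_Blueprint is a puzzle door wall that opens when light switches are turned on in the correct order.
; TurnOnLight advances an expected-number counter and calls OpenDoor once it reaches the Switchers count.
; An out-of-order on or off input resets the counter and sends TurnOffMessage to every switcher.
; OpenDoor locks out further input, enables mesh physics, nudges and tilts the wall, and plays audio.
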(event EventBeginPlay
  (Variables|Default|SetActualNumber 1))

(fn ConstructionScript)

(fn OpenDoor
  (bind _returnvalue (Transformation|GetActorLocation))
  (bind _returnvalue_2 (Transformation|GetActorRotation))
  (if (not (Variables|Default|GetIsOpen))
    (Variables|Default|SetIsOpen true)
    (Physics|SetSimulatePhysics (Variables|Debug|GetStaticMeshComponent) true)
    (Transformation|SetActorLocationAndRotation (Math|Vector|MakeVector (- (.x _returnvalue) 5e+01) (.y _returnvalue) (.z _returnvalue)) (Math|Rotator|MakeRotator 5.0 (.pitch _returnvalue_2) (.yaw _returnvalue_2)))
    (Audio|Components|Audio|Play (Variables|Default|GetAudio) 1e+01)))

(fn TurnonLight
  (params (Light :type Integer))
  (if (not (Variables|Default|GetIsOpen))
    (if (== Light (Variables|Default|GetActualNumber))
      (bind _result (Math|Integer|IncrementInt (Variables|Default|GetActualNumber))
        (:%20%20
          (bind _output_get (Variables|Default|SetActualNumber _result))
          (if (>= _output_get (Utilities|Array|Length (Variables|Default|GetSwitchers)))
            (CallFunction|OpenDoor))))
      (else
        (CallFunction|CleanLights)))))

(fn CleanLights
  (params (Actual :type Integer))
  (for _array_element (Variables|Default|GetSwitchers)
    (Class|BISwitch|TurnOff(Message) _array_element))
  (Variables|Default|SetActualNumber 1))

(fn TurnOffLight
  (params (Light :type Integer))
  (if (not (Variables|Default|GetIsOpen))
    (if (== Light (stale _result))
      (Variables|Default|SetActualNumber (stale _result))
      (else
        (CallFunction|CleanLights)))))