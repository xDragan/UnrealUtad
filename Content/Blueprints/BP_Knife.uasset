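; A grabbable knife that kills zombies on contact and reports the kill to the player.
; Grabbed turns off physics and snaps the knife to the grabber's sword_socket, while Dropped detaches it and restores physics and collision.
; When the Weapon component overlaps a BP_Zombie not already in the target state, it sets that state directly and calls KillZombie on player 0's BP_Player pawn.
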(event `/Game/Blueprints/BI_Grabbable.Grabbed`
  (params (GrabbedBy :type "SceneComponent Object Reference"))
  (`PrimitiveComponent.SetSimulatePhysics` (`self.StaticMeshComponent`) false)
  (`self.K2_AttachToComponent` GrabbedBy "sword_socket" "SnapToTarget" "SnapToTarget" "KeepWorld" false))

(event `/Game/Blueprints/BI_Grabbable.Dropped`
  (params (DroppedBy :type "SceneComponent Object Reference"))
  (`PrimitiveComponent.SetSimulatePhysics` (`self.StaticMeshComponent`) true)
  (`self.K2_DetachFromActor` "KeepWorld" "KeepWorld" "KeepWorld")
  (`PrimitiveComponent.SetCollisionEnabled` (`self.StaticMeshComponent`) "QueryAndPhysics"))

(event `self.Weapon.OnComponentBeginOverlap`
  (params (OverlappedComponent :type "PrimitiveComponent Object Reference") (OtherActor :type "Actor Object Reference") (OtherComp :type "PrimitiveComponent Object Reference") (OtherBodyIndex :type Integer) (bFromSweep :type Boolean) (SweepResult :type "HitResult Structure (by ref)"))
  (bind _asbp_zombie (cast `/Game/Blueprints/BP_Zombie` OtherActor))
  (if (`|EnumInequality` (`/Game/Blueprints/BP_Zombie.State` _asbp_zombie) "NewEnumerator5")
    (set `/Game/Blueprints/BP_Zombie.State` "NewEnumerator5" _asbp_zombie)
    (bind _asbp_player (cast `/Game/Blueprints/BP_Player` (`GameplayStatics.GetPlayerPawn` 0)))
    (`/Game/Blueprints/BP_Player.KillZombie` _asbp_player)))

(fn `UserConstructionScript`)