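; VR player pawn with locomotion, jumping, two-handed grabbing, a countdown display and an input to open a door.
; Tick moves the pawn along camera-relative input with optional acceleration, yaws the VR root and updates the remaining-time text.
; A ground overlap detector gates the impulse jump.
; Each hand grabs overlapping actors through BI_Grabbable messages, though both share a single GrabbedActor reference.
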(event `self.Ground Detector.OnComponentBeginOverlap`
  (params (OverlappedComponent :type "PrimitiveComponent Object Reference") (OtherActor :type "Actor Object Reference") (OtherComp :type "PrimitiveComponent Object Reference") (OtherBodyIndex :type Integer) (bFromSweep :type Boolean) (SweepResult :type "HitResult Structure (by ref)"))
  ;[1 1 1] Control de suelo
  (cast `/Game/Blueprints/BP_Player` OtherActor
    (:`CastFailed`
      (set `self.isGrounded` true))))

(event `self.Ground Detector.OnComponentEndOverlap`
  (params (OverlappedComponent :type "PrimitiveComponent Object Reference") (OtherActor :type "Actor Object Reference") (OtherComp :type "PrimitiveComponent Object Reference") (OtherBodyIndex :type Integer))
  ;[1 1 1] Control de suelo
  (cast `/Game/Blueprints/BP_Player` OtherActor
    (:`CastFailed`
      (set `self.isGrounded` false))))

(event `InputAction|Acceleration`
  (params (Key :type "Key Structure"))
  (:`Pressed`
    (set `self.IsAccelerated` true))
  (:`Released`
    (set `self.IsAccelerated` false)))

(event `InputAction|Grab Left`
  (params (Key :type "Key Structure"))
  (bind _lefthand (`self.LeftHand`))
  (:`Pressed`
    (`self.GrabStart` _lefthand)
    (set `self.LeftGrab` true))
  (:`Released`
    (`self.GrabEnd` _lefthand)
    (set `self.LeftGrab` false)))

(event `InputAction|Grab Right`
  (params (Key :type "Key Structure"))
  (bind _righthand (`self.RightHand`))
  (:`Pressed`
    (`self.GrabStart` _righthand)
    (set `self.RightGrab` true))
  (:`Released`
    (`self.GrabEnd` _righthand)
    (set `self.RightGrab` false)))

(event `self.ReceiveBeginPlay`
  ;[0.3371 1 0.5028] Inicialización
  (`HeadMountedDisplayFunctionLibrary.SetTrackingOrigin` "Floor")
  (bind _asbp_animation_hand (cast `/Game/Zombies/Models/hands/BP_Animation_Hand` (`SkeletalMeshComponent.GetAnimInstance` (`self.LeftHand`))))
  (set `self.LeftHandAnimation` _asbp_animation_hand)
  (bind _asbp_animation_hand_2 (cast `/Game/Zombies/Models/hands/BP_Animation_Hand` (`SkeletalMeshComponent.GetAnimInstance` (`self.RightHand`))))
  (set `self.RightHandAnimation` _asbp_animation_hand_2)
  (set `self.isGrounded` true))

(event `InputAction|Jump`
  (params (Key :type "Key Structure"))
  ;[1 1 1] Salto
  (:`Pressed`
    (if (`self.isGrounded`)
      (`PrimitiveComponent.AddImpulse` (`self.Capsule`) (0.0 0.0 450.0) "None" true))))

(event `self.ReceiveTick`
  (params (DeltaSeconds :type "Float (single-precision)"))
  (bind _returnvalue (`KismetMathLibrary.MaxInt64` (- (`self.LifeTime`) (`GameplayStatics.GetTimeSeconds`))))
  ;[1 1 1] Movimento
  (`self.Get Input`)
  (`self.Set Movement` DeltaSeconds)
  (`self.Set Rotation` DeltaSeconds)
  (if (!= (`self.LastTime`) _returnvalue)
    (bind _output_get (set `self.LastTime` _returnvalue))
    (bind _stringtime (`self.Get Remaining Seconds` _output_get))
    (`TextRenderComponent.K2_SetText` (`self.TextRender`) _stringtime)))

(event `InputAction|OpenDoor`
  (params (Key :type "Key Structure"))
  (:`Pressed`
    (bind _returnvalue (`GameplayStatics.GetActorOfClass` "/Game/BP_Door_Wall_Blueprint.BP_Door_Wall_Blueprint_C"))
    (`/Game/BP_Door_Wall_Blueprint.OpenDoor` _returnvalue)))

(fn `Get Input`
  (bind _camera (`self.Camera`))
  (bind (_returnvalue_x _returnvalue_y) (`KismetMathLibrary.BreakVector` (+ (* (`SceneComponent.GetForwardVector` _camera) (`self.GetInputAxisValue`)) (* (`SceneComponent.GetRightVector` _camera) (`self.GetInputAxisValue`)))))
  (set `self.Movement Direction` (`KismetMathLibrary.Normal` (`KismetMathLibrary.MakeVector` _returnvalue_x _returnvalue_y))))

(fn `Get Remaining Seconds`
  (params (Seconds :type Integer64))
  (returns (StringTime :type Text))
  (bind _returnvalue (/ Seconds 60))
  (return (`|FormatText` "{minutes}:{seconds}" (`KismetTextLibrary.Conv_Int64ToText` _returnvalue false true 2) (`KismetTextLibrary.Conv_Int64ToText` (- Seconds (* _returnvalue 60)) false true 2))))

(fn `GrabEnd`
  (params (Hand :type "SkeletalMeshComponent Object Reference"))
  (message `/Game/Blueprints/BI_Grabbable.Dropped` (`self.GrabbedActor`) Hand)
  (set `self.IsGrabSword` false)
  (set `self.GrabbedActor` null))

(fn `GrabStart`
  (params (Hand :type "SkeletalMeshComponent Object Reference"))
  (for _array_element (`PrimitiveComponent.GetOverlappingActors` Hand null)
    (cast `/Game/Blueprints/BI_Grabbable` _array_element)
    (`|ExecutionSequence`
      (:`then_0`
        (message `/Game/Blueprints/BI_Grabbable.Grabbed` _array_element Hand)
        (set `self.GrabbedActor` _array_element)
        (set `self.IsGrabSword` true))
      (:`then_1`
        (break)))))

(fn `Set Movement`
  (params (DeltaTime :type "Float (double-precision)"))
  (locals (SpeedFactor :type "Float (double-precision)" :default 1.0))
  (if (`self.IsAccelerated`)
    (set `local.SpeedFactor` 2.0)
    (else
      (set `local.SpeedFactor` 1.0)))
  (`self.K2_AddActorLocalOffset` (* (`self.Movement Direction`) (* DeltaTime (* (`local.SpeedFactor`) (`self.Movement Speed`))))))

(fn `Set Rotation`
  (params (`Delta Time` :type "Float (double-precision)"))
  (`SceneComponent.K2_AddWorldRotation` (`self.VR root`) (`KismetMathLibrary.MakeRotator` 0.0 0.0 (* (`self.GetInputAxisValue`) (`self.Rotation Speed`) `Delta Time`)) false true))

(fn `UserConstructionScript`)