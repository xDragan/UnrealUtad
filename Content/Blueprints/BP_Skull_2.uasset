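; BP_Skull_2 is a grabbable skull prop that acts as a weight for column-and-stair puzzle pieces.
; Grab turns off physics and snaps it to the grabber's sword_socket; drop detaches it and restores physics and collision.
; Its Box overlap with a BP_ColumnBase calls MoveStairAndColumn using the height from its ACHasWeight component, raising on begin and lowering on end.
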(event `/Game/Blueprints/BI_Grabbable.Grabbed`
  (params (GrabbedBy :type "SceneComponent Object Reference"))
  (`PrimitiveComponent.SetSimulatePhysics` (`self.StaticMeshComponent`) false)
  (`self.K2_AttachToComponent` GrabbedBy "sword_socket" "SnapToTarget" "SnapToTarget" "KeepWorld" false))

(event `/Game/Blueprints/BI_Grabbable.Dropped`
  (params (DroppedBy :type "SceneComponent Object Reference"))
  (`PrimitiveComponent.SetSimulatePhysics` (`self.StaticMeshComponent`) true)
  (`self.K2_DetachFromActor` "KeepWorld" "KeepWorld" "KeepWorld")
  (`PrimitiveComponent.SetCollisionEnabled` (`self.StaticMeshComponent`) "QueryAndPhysics"))

(event `self.Box.OnComponentBeginOverlap`
  (params (OverlappedComponent :type "PrimitiveComponent Object Reference") (OtherActor :type "Actor Object Reference") (OtherComp :type "PrimitiveComponent Object Reference") (OtherBodyIndex :type Integer) (bFromSweep :type Boolean) (SweepResult :type "HitResult Structure (by ref)"))
  (bind _asbp_column_base (cast `/Game/Blueprints/BP_ColumnBase` OtherActor))
  (bind _height (`/Game/Blueprints/BI_Has_Weight.GetHeight` (`self.AC_Has_Weight`)))
  (`/Game/Blueprints/BP_ColumnBase.MoveStairAndColumn` _asbp_column_base _height true))

(event `self.Box.OnComponentEndOverlap`
  (params (OverlappedComponent :type "PrimitiveComponent Object Reference") (OtherActor :type "Actor Object Reference") (OtherComp :type "PrimitiveComponent Object Reference") (OtherBodyIndex :type Integer))
  (bind _asbp_column_base (cast `/Game/Blueprints/BP_ColumnBase` OtherActor))
  (bind _height (`/Game/Blueprints/BI_Has_Weight.GetHeight` (`self.AC_Has_Weight`)))
  (`/Game/Blueprints/BP_ColumnBase.MoveStairAndColumn` _asbp_column_base _height false))

(fn `UserConstructionScript`)