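; BP_Stair is a stair actor that moves vertically toward a target world height.
; The ACZMovable member supplies the Target Z and Speed.
; Each Tick offsets the actor along its local up axis without sweeping, capping the step at the remaining distance so it does not overshoot.
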(event `self.ReceiveTick`
  (params (DeltaSeconds :type "Float (single-precision)"))
  (bind (_returnvalue_x _returnvalue_y _returnvalue_z) (`KismetMathLibrary.BreakVector` (`self.K2_GetActorLocation`)))
  (bind _ac_zmovable (`self.AC_ZMovable`))
  (bind _target (`/Game/Blueprints/AC_ZMovable.Target` _ac_zmovable))
  (bind _returnvalue (- _target _returnvalue_z))
  (if (!= _target _returnvalue_z)
    (`self.K2_AddActorLocalOffset` (* (`KismetMathLibrary.Vector_Up`) (* (`KismetMathLibrary.FMin` (`KismetMathLibrary.Abs` (* DeltaSeconds (`/Game/Blueprints/AC_ZMovable.Speed` _ac_zmovable))) (`KismetMathLibrary.Abs` _returnvalue)) (`KismetMathLibrary.SignOfFloat` _returnvalue))))))

(fn `UserConstructionScript`)