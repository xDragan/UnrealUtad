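; BP_Switch is an overlap-triggered switch that reports its on/off state to a door.
; On BeginPlay it starts off and caches the BP_Door_Wall_Blueprint actor it finds in the level.
; Each overlap toggles it, swaps the cube's material through EmitLight and calls the door's TurnOnLight or TurnOffLight with its Index.
; TurnOff and Turnon events set its state without notifying the door.
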(event `self.ReceiveActorBeginOverlap`
  (params (OtherActor :type "Actor Object Reference"))
  (bind _door (`self.Door`))
  (bind _index (`self.Index`))
  (if (`self.isTurnOn`)
    (`self.EmitLight` false)
    (set `self.isTurnOn` false)
    (`/Game/Blueprints/BP_Door_Wall_Blueprint.TurnOffLight` _door _index)
    (else
      (`self.EmitLight` true)
      (set `self.isTurnOn` true)
      (`/Game/Blueprints/BP_Door_Wall_Blueprint.TurnOnLight` _door _index))))

(event `self.ReceiveBeginPlay`
  (`self.EmitLight` false)
  (set `self.isTurnOn` false)
  (bind _returnvalue (`GameplayStatics.GetActorOfClass` "/Game/Blueprints/BP_Door_Wall_Blueprint.BP_Door_Wall_Blueprint_C"))
  (set `self.Door` _returnvalue))

(event `/Game/Blueprints/BI_Switch.TurnOff`
  (if (`self.isTurnOn`)
    (`self.EmitLight` false)
    (set `self.isTurnOn` false)))

(event `/Game/Blueprints/BI_Switch.TurnOn`
  (if (not (`self.isTurnOn`))
    (`self.EmitLight` true)
    (set `self.isTurnOn` true)))

(fn `EmitLight`
  (params (Enabled :type Boolean))
  (bind _cube (`self.Cube`))
  (if Enabled
    (`PrimitiveComponent.SetMaterial` _cube 0 (`self.MaterialOn`))
    (else
      (`PrimitiveComponent.SetMaterial` _cube 0 (`self.MaterialOff`)))))

(fn `UserConstructionScript`)