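; Behavior tree decorator for zombie AI that passes only when a target counts as visible.
; It casts the owner to AIC_Zombie and reads a distance float and a visibility bool from the blackboard.
; The check succeeds when the distance is above zero, within the controller's MaxVisibleDistance, and the visible flag is set.
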(fn `PerformConditionCheck`
  (params (OwnerActor :type "Actor Object Reference"))
  (returns (ReturnValue :type Boolean))
  (bind _returnvalue (`BTFunctionLibrary.GetBlackboardValueAsFloat` (`self.DistanceKey`)))
  (bind _asaic_zombie (cast `/Game/Blueprints/AIC_Zombie` OwnerActor))
  (return (and (> _returnvalue 0.0) (and (<= _returnvalue (`/Game/Blueprints/AIC_Zombie.MaxVisibleDistance` _asaic_zombie)) (`BTFunctionLibrary.GetBlackboardValueAsBool` (`self.VisibleKey`))))))