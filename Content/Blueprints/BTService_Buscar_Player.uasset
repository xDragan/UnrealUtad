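; Behavior tree service that updates an AI's facing and distance relative to the Blackboard target actor, likely the player.
; Each tick it flattens both locations to XY and writes their separation to DistanceKey.
; VisibleKey comes from the sign of a dot product between pawn forward and the target-to-pawn vector, so it is true when the target is behind.
; No line-of-sight check is made.
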(event `self.ReceiveTick`
  (params (OwnerActor :type "Actor Object Reference") (DeltaSeconds :type "Float (single-precision)"))
  (bind _asaicontroller (cast `AIController` OwnerActor))
  (bind _returnvalue (`Controller.K2_GetPawn` _asaicontroller))
  (bind _returnvalue_2 (- (`KismetMathLibrary.MakeVector` (.x (`Actor.K2_GetActorLocation` _returnvalue)) (.y (`Actor.K2_GetActorLocation` _returnvalue))) (`KismetMathLibrary.MakeVector` (.x (`Actor.K2_GetActorLocation` (`BTFunctionLibrary.GetBlackboardValueAsActor` (`self.TargetKey`)))) (.y (`Actor.K2_GetActorLocation` (`BTFunctionLibrary.GetBlackboardValueAsActor` (`self.TargetKey`)))))))
  (`BTFunctionLibrary.SetBlackboardValueAsBool` (`self.VisibleKey`) (> (`KismetMathLibrary.Dot_VectorVector` (`Actor.GetActorForwardVector` _returnvalue) _returnvalue_2) 0.0))
  (`BTFunctionLibrary.SetBlackboardValueAsFloat` (`self.DistanceKey`) (`KismetMathLibrary.VSize` _returnvalue_2)))